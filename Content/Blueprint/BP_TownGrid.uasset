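; Procedural town generator actor that scatters houses and roads on a grid at BeginPlay or through GenerateTown.
; It fills a free-position list from Row, Column and Offset, relative to its own X/Y.
; A random number of BP_House actors take random cells from that list.
; Each house then gets at most one BP_Road on a free orthogonal neighbour cell, found via a direction-to-offset map; a road connectivity check is left unwired.
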(event Custom|GenerateTown
  ;[1 1 1] Create a grid of random pos
  (CallFunction|GenerateDirection)
  (Utilities|Array|Clear (Variables|Grid|GetallFreePos))
  (Utilities|Array|Clear (Variables|HouseSpawn|GetallHouses))
  (for _index (range 0 (Variables|Grid|Getrow))
    (for _index_2 (range 0 (Variables|Grid|Getcolumn))
      (Utilities|Array|Add (Variables|Grid|GetallFreePos) (Math|Vector|MakeVector (+ (* (Math|Conversions|ToFloat(Integer) _index) (Variables|Grid|Getoffset)) (.x (.location (Transformation|GetActorTransform)))) (+ (* (Math|Conversions|ToFloat(Integer) _index_2) (Variables|Grid|Getoffset)) (.y (.location (Transformation|GetActorTransform)))) 0.0))))
  (CallFunction|SpawnHouses))

(event Custom|SpawnHouses
  ;[1 1 1] SpawnHouses
  (bind _output_get (Variables|HouseSpawn|SetNumberOfHouses (Math|Random|RandomIntegerinRange 5 (/ (Utilities|Array|Length (Variables|Grid|GetallFreePos)) 3))))
  (for _index (range 0 _output_get)
    (Variables|HouseSpawn|SetrandomHouse (.OutItem (Utilities|Array|Random (Variables|Grid|GetallFreePos))))
    (Game|SpawnActorfromClass "/Game/Blueprint/BP_House.BP_House_C" (Math|Transform|MakeTransform (Variables|HouseSpawn|GetrandomHouse)) "Undefined" "MultiplyWithRoot" 0 0)
    (Utilities|Array|Add (Variables|HouseSpawn|GetallHouses) (Variables|HouseSpawn|GetrandomHouse))
    (Utilities|Array|RemoveItem (Variables|Grid|GetallFreePos) (Variables|HouseSpawn|GetrandomHouse)))
  (CallFunction|SpawnRoad))

(event Custom|SpawnRoad
  (bind _array_element (Utilities|Array|ForEachLoopwithBreak (Variables|HouseSpawn|GetallHouses))
    (:LoopBody
      (Variables|RoadSpawn|SethousePos _array_element)
      (bind _array_element_2 (Utilities|Array|ForEachLoopwithBreak (Variables|Grid|GetallFreePos))
        (:LoopBody
          (Variables|RoadSpawn|SetfreePos _array_element_2)
          (if (Utilities|CheckAvailablePosatDirection "NewEnumerator3")
            (CallFunction|BreakSpawnOneRoad true)
            (elif (Utilities|CheckAvailablePosatDirection "NewEnumerator1")
              (CallFunction|BreakSpawnOneRoad true)
              (elif (Utilities|CheckAvailablePosatDirection "NewEnumerator2")
                (CallFunction|BreakSpawnOneRoad true)
                (elif (Utilities|CheckAvailablePosatDirection "NewEnumerator0")
                  (CallFunction|BreakSpawnOneRoad true))))))))))

(event Custom|BreakSpawnOneRoad
  (params (SpawnRoad :type Boolean))
  (if SpawnRoad
    (CallFunction|SpawnNewRoad)
    (Utilities|Array|ForEachLoopwithBreak (Variables|Grid|GetallFreePos)) ; enters at Break
    (else
      (Utilities|Array|ForEachLoopwithBreak (Variables|Grid|GetallFreePos)) ; enters at Break
    )))

(event EventBeginPlay
  ;[1 1 1] Create a grid of random pos
  (CallFunction|GenerateDirection)
  (Utilities|Array|Clear (Variables|Grid|GetallFreePos))
  (Utilities|Array|Clear (Variables|HouseSpawn|GetallHouses))
  (for _index (range 0 (Variables|Grid|Getrow))
    (for _index_2 (range 0 (Variables|Grid|Getcolumn))
      (Utilities|Array|Add (Variables|Grid|GetallFreePos) (Math|Vector|MakeVector (+ (* (Math|Conversions|ToFloat(Integer) _index) (Variables|Grid|Getoffset)) (.x (.location (Transformation|GetActorTransform)))) (+ (* (Math|Conversions|ToFloat(Integer) _index_2) (Variables|Grid|Getoffset)) (.y (.location (Transformation|GetActorTransform)))) 0.0))))
  (CallFunction|SpawnHouses))

(fn ConstructionScript)

(fn GenerateDirection
  (bind _result (Math|Float|NegateFloat (Variables|Grid|Getoffset))
    (:%20%20
      (Utilities|Map|Add (Variables|Default|Getdirection) "NewEnumerator0" (Math|Vector|MakeVector _result 0.0 0.0))
      (Utilities|Map|Add (Variables|Default|Getdirection) "NewEnumerator3" (Math|Vector|MakeVector (Variables|Grid|Getoffset) 0.0 0.0))
      (Utilities|Map|Add (Variables|Default|Getdirection) "NewEnumerator1" (Math|Vector|MakeVector 0.0 (Variables|Grid|Getoffset) 0.0))
      (bind _result_2 (Math|Float|NegateFloat (Variables|Grid|Getoffset))
        (:%20%20
          (Utilities|Map|Add (Variables|Default|Getdirection) "NewEnumerator2" (Math|Vector|MakeVector 0.0 _result_2 0.0)))))))

(fn SpawnNewRoad
  (Game|SpawnActorfromClass "/Game/Blueprint/BP_Road.BP_Road_C" (Math|Transform|MakeTransform (Variables|RoadSpawn|GetfreePos)) "Undefined" "MultiplyWithRoot" 0 0)
  (Utilities|Array|Add (Variables|RoadSpawn|GetallRoads) (Variables|RoadSpawn|GetfreePos))
  (Utilities|Array|RemoveItem (Variables|Grid|GetallFreePos) (Variables|RoadSpawn|GetfreePos)))