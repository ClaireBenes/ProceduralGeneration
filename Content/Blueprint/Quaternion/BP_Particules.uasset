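; Actor that moves its Particles component along a parametric rose curve in its local YZ plane.
; Each Tick, time since creation scaled by Speed feeds Rose, whose sine and cosine products form an eight-petal pattern scaled by PatternSize.
; Abstract and Infinite hold alternative curve formulas that do not drive the movement, and an actor rotation node is left unexecuted.
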(event EventTick
  (params (DeltaSeconds :type Float%20%28single-precision%29))
  (bind _returnvalue (Actor|GetGameTimeSinceCreation))
  (bind _speed (Variables|Default|GetSpeed))
  (bind _patternsize (Variables|Default|GetpatternSize))
  (bind _returnvalue_2 (* _returnvalue _speed))
  (bind (_y _z) (Utilities|Rose _returnvalue_2))
  (Transformation|SetRelativeLocation (Variables|Default|GetParticles) (Math|Vector|MakeVector 0.0 (* _y _patternsize) (* _patternsize _z)) false false))

(fn ConstructionScript)