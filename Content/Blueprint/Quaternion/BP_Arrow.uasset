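; BP_Arrow is an actor that rotates in fixed steps from player input, apparently as a quaternion rotation demo.
; On BeginPlay it adds the IMC_Second mapping context to player 0.
; IA_RotX, IA_RotY and IA_RotZ each build an axis quaternion from half-angle sine and cosine of Angle.
; Right-multiplying the actor's rotation by it, or its inverse for non-positive input, turns the actor about its local axis.
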(event Input|EnhancedActionEvents|EnhancedInputActionIA_RotX
  (params (ActionValue :type Float%20%28double-precision%29) (ElapsedSeconds :type Float%20%28double-precision%29) (TriggeredSeconds :type Float%20%28double-precision%29) (InputAction :type Input%20Action%20Object%20Reference :default "/Game/Input/IA_RotX.IA_RotX"))
  (bind _returnvalue (Transformation|GetActorRotation))
  (bind _angle (Variables|Default|Getangle))
  (bind _returnvalue_2 (Math|Conversions|ToQuaternion(Rotator) _returnvalue))
  (bind _returnvalue_3 (/ _angle 2.0))
  (bind _returnvalue_4 (Math|Trig|Sin(Degrees) _returnvalue_3))
  (bind _returnvalue_5 (Math|Trig|Cos(Degrees) _returnvalue_3))
  (bind _returnvalue_6 (Class|KismetMathLibrary|MakeQuat _returnvalue_4 0.0 0.0 _returnvalue_5))
  (:Started
    (Transformation|SetActorRotation (Math|Rotator|SelectRotator (Class|KismetMathLibrary|QuatRotator (* _returnvalue_2 _returnvalue_6)) (Class|KismetMathLibrary|QuatRotator (* _returnvalue_2 (Class|KismetMathLibrary|QuatInversed _returnvalue_6))) (> ActionValue 0.0)))))

(event Input|EnhancedActionEvents|EnhancedInputActionIA_RotY
  (params (ActionValue :type Float%20%28double-precision%29) (ElapsedSeconds :type Float%20%28double-precision%29) (TriggeredSeconds :type Float%20%28double-precision%29) (InputAction :type Input%20Action%20Object%20Reference :default "/Game/Input/IA_RotY.IA_RotY"))
  (bind _returnvalue (Transformation|GetActorRotation))
  (bind _angle (Variables|Default|Getangle))
  (bind _returnvalue_2 (Math|Conversions|ToQuaternion(Rotator) _returnvalue))
  (bind _returnvalue_3 (/ _angle 2.0))
  (bind _returnvalue_4 (Math|Trig|Sin(Degrees) _returnvalue_3))
  (bind _returnvalue_5 (Math|Trig|Cos(Degrees) _returnvalue_3))
  (bind _returnvalue_6 (Class|KismetMathLibrary|MakeQuat 0.0 _returnvalue_4 0.0 _returnvalue_5))
  (:Started
    (Transformation|SetActorRotation (Math|Rotator|SelectRotator (Class|KismetMathLibrary|QuatRotator (* _returnvalue_2 _returnvalue_6)) (Class|KismetMathLibrary|QuatRotator (* _returnvalue_2 (Class|KismetMathLibrary|QuatInversed _returnvalue_6))) (> ActionValue 0.0)))))

(event Input|EnhancedActionEvents|EnhancedInputActionIA_RotZ
  (params (ActionValue :type Float%20%28double-precision%29) (ElapsedSeconds :type Float%20%28double-precision%29) (TriggeredSeconds :type Float%20%28double-precision%29) (InputAction :type Input%20Action%20Object%20Reference :default "/Game/Input/IA_RotZ.IA_RotZ"))
  (bind _returnvalue (Transformation|GetActorRotation))
  (bind _angle (Variables|Default|Getangle))
  (bind _returnvalue_2 (Math|Conversions|ToQuaternion(Rotator) _returnvalue))
  (bind _returnvalue_3 (/ _angle 2.0))
  (bind _returnvalue_4 (Math|Trig|Sin(Degrees) _returnvalue_3))
  (bind _returnvalue_5 (Math|Trig|Cos(Degrees) _returnvalue_3))
  (bind _returnvalue_6 (Class|KismetMathLibrary|MakeQuat 0.0 0.0 _returnvalue_4 _returnvalue_5))
  (:Started
    (Transformation|SetActorRotation (Math|Rotator|SelectRotator (Class|KismetMathLibrary|QuatRotator (* _returnvalue_2 _returnvalue_6)) (Class|KismetMathLibrary|QuatRotator (* _returnvalue_2 (Class|KismetMathLibrary|QuatInversed _returnvalue_6))) (> ActionValue 0.0)))))

(event EventBeginPlay
  (bind _returnvalue (Game|GetPlayerController 0))
  (bind _returnvalue_2 (PlayerController|LocalPlayerSubsystems|GetEnhancedInputLocalPlayerSubsystem _returnvalue))
  (Utilities|IsValid _returnvalue_2
    (:Is%20Valid
      (Input|AddMappingContext _returnvalue_2 "/Game/Input/IMC_Second.IMC_Second" 0 "(bIgnoreAllPressedKeysUntilRelease=True,bForceImmediately=False,bNotifyUserSettings=False)"))))

(event Collision|EventActorBeginOverlap
  (params (OtherActor :type Actor%20Object%20Reference)))

(event EventTick
  (params (DeltaSeconds :type Float%20%28single-precision%29)))

(fn ConstructionScript)