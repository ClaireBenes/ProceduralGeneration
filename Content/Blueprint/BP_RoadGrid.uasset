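; BP_RoadGrid procedurally lays out a town road network on a grid of BP_Road actors, on BeginPlay or GenerateTown.
; It fills a free-position list from its location, then repeatedly picks random endpoint pairs.
; LinkRoads recursively steps from first toward second, randomly choosing X or Y, spawning roads until it hits a recorded endpoint.
; Intermediate cells are never recorded, and the Direction map from GenerateDirection is unused here.
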(event Custom|GenerateTown
  ;[1 1 1] Create a grid of random pos
  (CallFunction|GenerateDirection)
  (Utilities|Array|Clear (Variables|Roads|GetallRoads))
  (Utilities|Array|Clear (Variables|Default|GetallFreePos))
  (for _index (range 0 (Variables|Grid|Getrow))
    (for _index_2 (range 0 (Variables|Grid|Getcolumn))
      (Utilities|Array|Add (Variables|Default|GetallFreePos) (Math|Vector|MakeVector (+ (* (Math|Conversions|ToFloat(Integer) _index) (Variables|Grid|Getoffset)) (.x (.location (Transformation|GetActorTransform)))) (+ (* (Math|Conversions|ToFloat(Integer) _index_2) (Variables|Grid|Getoffset)) (.y (.location (Transformation|GetActorTransform)))) 0.0))))
  (CallFunction|SpawnRoad))

(event Custom|SpawnRoad
  (bind _allfreepos (Variables|Default|GetallFreePos))
  (bind _outitem (Utilities|Array|Random _allfreepos))
  ;[1 1 1] Spawn first 2 roads (for x number of times)
  (for _index (range 0 5)
    (Variables|Roads|SetfirstRoad _outitem)
    (Variables|Roads|SetsecondRoad _outitem)
    (Game|SpawnActorfromClass "/Game/Blueprint/BP_Road.BP_Road_C" (Math|Transform|MakeTransform (Variables|Roads|GetfirstRoad) "0, 0, 0" "3.500000,3.500000,1.000000") "Undefined" "MultiplyWithRoot" 0 0)
    (Utilities|Array|Add (Variables|Roads|GetallRoads) (Variables|Roads|GetfirstRoad))
    (Utilities|Array|RemoveItem (Variables|Default|GetallFreePos) (Variables|Roads|GetfirstRoad))
    (Utilities|Array|Add (Variables|Roads|GetallRoads) (Variables|Roads|GetsecondRoad))
    (Utilities|Array|RemoveItem (Variables|Default|GetallFreePos) (Variables|Roads|GetsecondRoad))
    (Variables|Roads|Setorigin (Variables|Roads|GetfirstRoad))
    (CallFunction|LinkRoads)))

(event Custom|LinkRoads
  ;[1 1 1] Spawn Next Road
  (Utilities|Array|Clear (Variables|Pathfinding|GetpossibleDirection))
  (bind _output_get (Variables|Pathfinding|SetvectorDirection (- (Variables|Roads|GetsecondRoad) (Variables|Roads|Getorigin))))
  (if (!= (Math|Float|Sign(Float) (.x _output_get)) 0.0)
    (Utilities|Array|Add (Variables|Pathfinding|GetpossibleDirection) (Math|Vector2D|MakeVector2D (Math|Float|Sign(Float) (.x _output_get)) 0.0)))
  (if (!= (Math|Float|Sign(Float) (.y _output_get)) 0.0)
    (Utilities|Array|Add (Variables|Pathfinding|GetpossibleDirection) (Math|Vector2D|MakeVector2D 0.0 (Math|Float|Sign(Float) (.y _output_get)))))
  (Variables|Pathfinding|SetdirectionToGo (.OutItem (Utilities|Array|Random (Variables|Pathfinding|GetpossibleDirection))))
  (Variables|Pathfinding|SetnewPos (+ (Variables|Roads|Getorigin) (* (Math|Vector|MakeVector (.x (Variables|Pathfinding|GetdirectionToGo)) (.y (Variables|Pathfinding|GetdirectionToGo)) 0.0) (Variables|Grid|Getoffset))))
  (if (== (Utilities|Array|FindItem (Variables|Roads|GetallRoads) (Variables|Pathfinding|GetnewPos)) -1)
    (Game|SpawnActorfromClass "/Game/Blueprint/BP_Road.BP_Road_C" (Math|Transform|MakeTransform (+ (Variables|Roads|Getorigin) (* (Math|Vector|MakeVector (.x (Variables|Pathfinding|GetdirectionToGo)) (.y (Variables|Pathfinding|GetdirectionToGo)) 0.0) (Variables|Grid|Getoffset))) "0, 0, 0" "3.500000,3.500000,1.000000") "Undefined" "MultiplyWithRoot" 0 0)
    (Utilities|Array|Add (Variables|Roads|GetallRoads) (Variables|Roads|GetsecondRoad))
    (Utilities|Array|RemoveItem (Variables|Default|GetallFreePos) (Variables|Roads|GetsecondRoad))
    ;[1 1 1] Create next road
    (Variables|Roads|Setorigin (Variables|Pathfinding|GetnewPos))
    (if (Utilities|Operators|NotEqual(!=) (Variables|Roads|Getorigin) (Variables|Roads|GetsecondRoad) 0.0)
      (CallFunction|LinkRoads))))

(event EventBeginPlay
  ;[1 1 1] Create a grid of random pos
  (CallFunction|GenerateDirection)
  (Utilities|Array|Clear (Variables|Roads|GetallRoads))
  (Utilities|Array|Clear (Variables|Default|GetallFreePos))
  (for _index (range 0 (Variables|Grid|Getrow))
    (for _index_2 (range 0 (Variables|Grid|Getcolumn))
      (Utilities|Array|Add (Variables|Default|GetallFreePos) (Math|Vector|MakeVector (+ (* (Math|Conversions|ToFloat(Integer) _index) (Variables|Grid|Getoffset)) (.x (.location (Transformation|GetActorTransform)))) (+ (* (Math|Conversions|ToFloat(Integer) _index_2) (Variables|Grid|Getoffset)) (.y (.location (Transformation|GetActorTransform)))) 0.0))))
  (CallFunction|SpawnRoad))

(fn ConstructionScript)

(fn GenerateDirection
  (bind _result (Math|Float|NegateFloat (Variables|Grid|Getoffset))
    (:%20%20
      (Utilities|Map|Add (Variables|Default|Getdirection) "NewEnumerator0" (Math|Vector|MakeVector _result 0.0 0.0))
      (Utilities|Map|Add (Variables|Default|Getdirection) "NewEnumerator3" (Math|Vector|MakeVector (Variables|Grid|Getoffset) 0.0 0.0))
      (Utilities|Map|Add (Variables|Default|Getdirection) "NewEnumerator1" (Math|Vector|MakeVector 0.0 (Variables|Grid|Getoffset) 0.0))
      (bind _result_2 (Math|Float|NegateFloat (Variables|Grid|Getoffset))
        (:%20%20
          (Utilities|Map|Add (Variables|Default|Getdirection) "NewEnumerator2" (Math|Vector|MakeVector 0.0 _result_2 0.0)))))))