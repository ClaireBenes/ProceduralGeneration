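; BP_Grid is an actor whose GenerateMaze event rebuilds a grid of BP_GridZone actors over Row and Column index ranges.
; It finds an existing zone as a size reference, then destroys and clears those tracked in AllZones.
; Nested loops spawn and track new zones from the grid's XY location at world Z zero.
; Spacing is four times the reference cube mesh's extent, using X for rows and Z for columns.
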(event Custom|GenerateMaze
  (bind _returnvalue (Transformation|GetActorLocation))
  (bind _allzones (Variables|Default|GetallZones))
  (bind _returnvalue_2 (Actor|GetActorOfClass "/Game/Blueprint/Grid/BP_GridZone.BP_GridZone_C"))
  (Variables|Default|SetObjectToSpawn _returnvalue_2)
  (for _array_element _allzones
    (Actor|DestroyActor _array_element))
  (Utilities|Array|Clear _allzones)
  (for _index (range 0 (Variables|Default|Getrow))
    (for _index_2 (range 0 (Variables|Default|Getcolumn))
      (bind _returnvalue_3 (Game|SpawnActorfromClass "/Game/Blueprint/Grid/BP_GridZone.BP_GridZone_C" (Math|Transform|MakeTransform (Math|Vector|MakeVector (+ (* (Math|Conversions|ToFloat(Integer) _index) (* (.x (.boxextent (StaticMesh|GetBounds (Variables|/Script/Engine.StaticMeshComponent|GetStaticMesh (Variables|/Game/Blueprint/Grid/BP_GridZone.BP_GridZone_C|GetCube (Variables|Default|GetObjectToSpawn)))))) 4.0)) (.x _returnvalue)) (+ (* (Math|Conversions|ToFloat(Integer) _index_2) (* (.z (.boxextent (StaticMesh|GetBounds (Variables|/Script/Engine.StaticMeshComponent|GetStaticMesh (Variables|/Game/Blueprint/Grid/BP_GridZone.BP_GridZone_C|GetCube (Variables|Default|GetObjectToSpawn)))))) 4.0)) (.y _returnvalue)) 0.0)) "Undefined" "MultiplyWithRoot" 0 0))
      (Utilities|Array|Add (Variables|Default|GetallZones) _returnvalue_3))))

(fn ConstructionScript)